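; BP_PlayerControllerTest is a test player controller that puts an on-screen terminal widget in front of the player.
; On BeginPlay it creates WBP_Terminal and adds it to the viewport.
; Text-updated and write-line events from its Terminal member set the widget's last line or append a new one.
; Tab toggles the Terminal between activated and deactivated through an Active flag, printing a debug string on each press.
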(event `self.ReceiveBeginPlay`
  (bind _returnvalue (`|CreateWidget` "/Game/AADeveloping/Widgets/WBP_Terminal.WBP_Terminal_C" self))
  (bind _output_get (set `self.WBP_Terminal` _returnvalue))
  (`UserWidget.AddToViewport` _returnvalue 0)
  (`UserWidget.AddToViewport` _output_get 0))

(event `self.Terminal.TextUpdated`
  (params (Text :type String))
  (bind _wbp_terminal (`self.WBP_Terminal`)
    (:`then`
      (`/Game/AADeveloping/Widgets/WBP_Terminal.SetLastLineText` _wbp_terminal Text))
    (:`else`)))

(event `self.Terminal.TextWriteLine`
  (params (Text :type String))
  (bind _wbp_terminal (`self.WBP_Terminal`)
    (:`then`
      (`/Game/AADeveloping/Widgets/WBP_Terminal.AddNewLineText` _wbp_terminal Text))
    (:`else`)))

(event `Key|Tab`
  (params (Key :type "Key Structure"))
  (bind _terminal (`self.Terminal`))
  (:`Pressed`
    (`KismetSystemLibrary.PrintString` "Hello")
    (if (`self.bActive`)
      (`Terminal.DeactivateTerminal` _terminal)
      (set `self.bActive` false)
      (else
        (`Terminal.ActivateTerminal` _terminal)
        (set `self.bActive` true)))))

(fn `UserConstructionScript`)