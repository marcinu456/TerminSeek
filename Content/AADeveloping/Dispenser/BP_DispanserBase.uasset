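; Base dispenser actor that hands items to the player and can require repair.
; An overlap collision registers it as the character's current actor; on use it spawns an item of its ItemType attached to the character's left-hand socket if empty-handed.
; When NeedRepair is set, use opens the controller's repair widget, and OnRepair sets Health from the success count.
; On BeginPlay, a light cube's material reflects cooldown state.
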(event `self.ReceiveBeginPlay`
  (`self.UpdateDispenserStatusInfo`))

(event `self.InteractiveCollison.OnComponentBeginOverlap`
  (params (OverlappedComponent :type "PrimitiveComponent Object Reference") (OtherActor :type "Actor Object Reference") (OtherComp :type "PrimitiveComponent Object Reference") (OtherBodyIndex :type Integer) (bFromSweep :type Boolean) (SweepResult :type "HitResult Structure (by ref)"))
  (bind _asbp_third_person_character (cast `/Game/ThirdPerson/Blueprints/BP_ThirdPersonCharacter` OtherActor))
  (set `/Game/ThirdPerson/Blueprints/BP_ThirdPersonCharacter.BPCurrentActorHold` self _asbp_third_person_character))

(event `self.InteractiveCollison.OnComponentEndOverlap`
  (params (OverlappedComponent :type "PrimitiveComponent Object Reference") (OtherActor :type "Actor Object Reference") (OtherComp :type "PrimitiveComponent Object Reference") (OtherBodyIndex :type Integer))
  (bind _asbp_third_person_character (cast `/Game/ThirdPerson/Blueprints/BP_ThirdPersonCharacter` OtherActor))
  (set `/Game/ThirdPerson/Blueprints/BP_ThirdPersonCharacter.BPCurrentActorHold` null _asbp_third_person_character))

(event `/Game/AADeveloping/Dispenser/BPI_ItemInterface.OnUse`
  (params (Character :type "Actor Object Reference"))
  (bind _asbp_third_person_character (cast `/Game/ThirdPerson/Blueprints/BP_ThirdPersonCharacter` Character))
  (if (and (not (`/Game/ThirdPerson/Blueprints/BP_ThirdPersonCharacter.bIsHolding` _asbp_third_person_character)) (not (`self.bNeedRepair`)))
    (bind _returnvalue (`|SpawnActorFromClass` "/Game/AADeveloping/Dispenser/BP_ItemBase.BP_ItemBase_C" (`self.GetTransform`) "Undefined" "MultiplyWithRoot" null (`self.ItemType`) null))
    (bind _returnvalue_2 (`self.K2_AttachToComponent` _returnvalue (`Character.Mesh` _asbp_third_person_character) "hand_lSocket" "SnapToTarget" "KeepRelative" "KeepRelative" true))
    (set `/Game/ThirdPerson/Blueprints/BP_ThirdPersonCharacter.bIsHolding` _returnvalue_2 _asbp_third_person_character)
    (set `/Game/ThirdPerson/Blueprints/BP_ThirdPersonCharacter.BPCurrentHoldItem` _returnvalue _asbp_third_person_character)
    (elif (`self.bNeedRepair`)
      (bind _asbp_player_controller_test (cast `/Game/AADeveloping/BP_PlayerControllerTest` (`GameplayStatics.GetPlayerController` 0)))
      (`/Game/AADeveloping/BP_PlayerControllerTest.CreateRepairWidget` _asbp_player_controller_test self))))

(event `/Game/AADeveloping/Dispenser/BPI_ItemInterface.OnRepair`
  (params (NumberOfSucces :type Integer))
  (set `self.Health` (`KismetMathLibrary.Conv_IntToDouble` (* NumberOfSucces 25))))

(fn `UpdateDispenserStatusInfo`
  (`self.UpdateLight`))

(fn `UpdateLight`
  (bind _lightcubeinfo (`self.LightCubeInfo`))
  (if (`self.bIsCoolDown`)
    (`PrimitiveComponent.SetMaterial` _lightcubeinfo 0 "/Game/AADeveloping/Dispenser/LightInfoCoolDown.LightInfoCoolDown")
    (else
      (`PrimitiveComponent.SetMaterial` _lightcubeinfo 0 "/Game/AADeveloping/Dispenser/LightInfoMat.LightInfoMat"))))

(fn `UserConstructionScript`)