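; BP_DispenserTrash is a trash dispenser actor that disposes of whatever object a player character is carrying when used.
; On use, it casts the user to BP_ThirdPersonCharacter and, if that character is holding something, calls RemoveHoldingObject on it.
; Tick resets Health to a fixed value every frame, so damage to the dispenser does not accumulate.
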(event `self.ReceiveTick`
  (params (DeltaSeconds :type "Float (single-precision)"))
  (set `self.Health` 100.0))

(event `/Game/AADeveloping/Dispenser/BPI_ItemInterface.OnUse`
  (params (Character :type "Actor Object Reference"))
  (bind _asbp_third_person_character (cast `/Game/ThirdPerson/Blueprints/BP_ThirdPersonCharacter` Character))
  (if (`/Game/ThirdPerson/Blueprints/BP_ThirdPersonCharacter.bIsHolding` _asbp_third_person_character)
    (`/Game/ThirdPerson/Blueprints/BP_ThirdPersonCharacter.RemoveHoldingObject` _asbp_third_person_character)))

(fn `UserConstructionScript`
  (`parent.UserConstructionScript`))