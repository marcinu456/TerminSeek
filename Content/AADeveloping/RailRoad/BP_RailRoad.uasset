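; BP_RailRoad is a railroad actor that builds twin rails along an editable spline in its Construction Script; the Event Graph is unused.
; A loop advances Distance by SegmentLeght, adding two spline mesh components per step, offset to either side along the spline's right vector by WildCart.
; Segments use unit direction vectors as tangents, and any remainder at the spline's end not exceeding one segment length stays empty.
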(fn `UserConstructionScript`
  (locals (Distance :type "Float (double-precision)") (SegmentLeght :type "Float (double-precision)" :default 50.0) (WildCart :type "Float (single-precision)" :default 250.0))
  (bind _spline (`self.Spline`))
  (bind _distance (`local.Distance`))
  (bind _spline_2 (`self.Spline`))
  (bind _wildcart (`local.WildCart`))
  (bind _wildcart_2 (`local.WildCart`))
  (bind _returnvalue (`SplineComponent.GetLocationAtDistanceAlongSpline` _spline_2 _distance "Local"))
  (bind _returnvalue_2 (`SplineComponent.GetDirectionAtDistanceAlongSpline` _spline_2 _distance "Local"))
  (bind _returnvalue_3 (`SplineComponent.GetRightVectorAtDistanceAlongSpline` _spline_2 _distance "Local"))
  (bind _returnvalue_4 (+ (`local.Distance`) (`local.SegmentLeght`)))
  (bind _returnvalue_5 (`SplineComponent.GetLocationAtDistanceAlongSpline` _spline _returnvalue_4 "Local"))
  (bind _returnvalue_6 (`SplineComponent.GetDirectionAtDistanceAlongSpline` _spline _returnvalue_4 "Local"))
  (bind _returnvalue_7 (`SplineComponent.GetRightVectorAtDistanceAlongSpline` _spline _returnvalue_4 "Local"))
  (if (> (`SplineComponent.GetSplineLength` (`self.Spline`)) _returnvalue_4) :!label _label
    (`|ExecutionSequence`
      (:`then_0`
        (bind _returnvalue_8 (`AddComponent|NODE_AddSplineMeshComponent-0`))
        (`SplineMeshComponent.SetStartAndEnd` _returnvalue_8 (+ _returnvalue (* _returnvalue_3 _wildcart_2)) _returnvalue_2 (+ _returnvalue_5 (* _returnvalue_7 _wildcart)) _returnvalue_6 true)
        (bind _returnvalue_9 (`AddComponent|NODE_AddSplineMeshComponent-1`))
        (`SplineMeshComponent.SetStartAndEnd` _returnvalue_9 (+ _returnvalue (* _returnvalue_3 (* _wildcart_2 -1.0))) _returnvalue_2 (+ _returnvalue_5 (* _returnvalue_7 (* _wildcart -1.0))) _returnvalue_6 true))
      (:`then_1`
        (set `local.Distance` _returnvalue_4)
        (goto _label)))))