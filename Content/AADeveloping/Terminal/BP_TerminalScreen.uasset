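; BP_TerminalScreen is an in-world terminal screen actor that displays terminal text on a text render component.
; It enables input from player controller 0 on BeginPlay, and Tab toggles its Terminal component between activated and deactivated via an Active flag, printing a debug "Hello" on each press.
; The Terminal's TextUpdated event pushes each new string into TerminalTextRender.
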(event `self.ReceiveBeginPlay`
  (`self.EnableInput` (`GameplayStatics.GetPlayerController` 0)))

(event `self.Terminal.TextUpdated`
  (params (Text :type String))
  (`TextRenderComponent.K2_SetText` (`self.TerminalTextRender`) (`KismetTextLibrary.Conv_StringToText` Text)))

(event `Key|Tab`
  (params (Key :type "Key Structure"))
  (bind _terminal (`self.Terminal`))
  (:`Pressed`
    (`KismetSystemLibrary.PrintString` "Hello")
    (if (`self.bActive`)
      (`Terminal.DeactivateTerminal` _terminal)
      (set `self.bActive` false)
      (else
        (`Terminal.ActivateTerminal` _terminal)
        (set `self.bActive` true)))))

(fn `UserConstructionScript`)