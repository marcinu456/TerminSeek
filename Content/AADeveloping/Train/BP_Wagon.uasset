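; BP_Wagon is a train wagon that fills some of its seats with passengers when play begins.
; It collects BP_WagonSeat child actors, then after a short delay reads difficulty from BP_GameInstance to set the passenger count, higher on harder settings.
; It draws random seats from a working array, removing each pick to avoid repeats, though the random range's upper bound overshoots the last index by one.
; The picked seats are then enabled.
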(event `self.ReceiveBeginPlay`
  (`self.AddSeatsToArray`)
  (`KismetSystemLibrary.Delay` 0.2)
  (`self.SpawmPassengersInWagon`))

(fn `AddSeatsToArray`
  (for _array_element (`self.K2_GetComponentsByClass` "/Script/Engine.ChildActorComponent")
    (bind _asbp_wagon_seat (cast `/Game/AADeveloping/Train/BP_WagonSeat` (`ChildActorComponent.ChildActor` _array_element)))
    (`KismetArrayLibrary.Array_Add` (`self.Seats`) _asbp_wagon_seat)))

(fn `SpawmPassengersInWagon`
  (locals (PassengersToSpawn :type Integer) (RefPassengers :type "Array of /Game/AADeveloping/Train/BP_WagonSeat Object Reference") (PassengerToSeat :type "Array of /Game/AADeveloping/Train/BP_WagonSeat Object Reference") (CurrentNumber :type Integer :default 0))
  (bind _refpassengers (`local.RefPassengers`))
  (set `local.RefPassengers` (`self.Seats`))
  (`|ExecutionSequence`
    (:`then_0`
      (bind _asbp_game_instance (cast `/Game/AADeveloping/BP_GameInstance` (`GameplayStatics.GetGameInstance`)))
      (set `local.PassengersToSpawn` (select `/Game/AADeveloping/Menu/E_Difficulty` (`/Game/AADeveloping/BP_GameInstance.Difficult` _asbp_game_instance) :`NewEnumerator0` 4 :`NewEnumerator1` 6 :`NewEnumerator2` 9)))
    (:`then_1`
      (while (> (`local.PassengersToSpawn`) 0)
        (bind _output_get (set `local.CurrentNumber` (`KismetMathLibrary.RandomIntegerInRange` 0 (- (`KismetArrayLibrary.Array_Length` (`local.RefPassengers`)) 0))))
        (`KismetArrayLibrary.Array_Add` (`local.PassengerToSeat`) (`|GetArrayItem` _refpassengers _output_get))
        (`KismetArrayLibrary.Array_Remove` _refpassengers _output_get)
        (`/Engine/EditorBlueprintResources/StandardMacros.DecrementInt` (`local.PassengersToSpawn`)))
      (for _array_element (`local.PassengerToSeat`)
        (`/Game/AADeveloping/Train/BP_WagonSeat.SetSeatEnabled` _array_element true)))))

(fn `UserConstructionScript`)